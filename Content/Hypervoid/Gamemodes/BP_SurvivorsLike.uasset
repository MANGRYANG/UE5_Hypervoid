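; Survivors-like game mode that adds a timer widget, plays background music and runs timed enemy waves around the player.
; Tick accumulates play time and spawns drone batches at random offsets, sized by a time-based formula, while the spawn period is always evaluated at time zero.
; After four minutes it spawns two distant middle bosses, then a giant last boss ahead of the player whenever neither boss type remains.
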(event EventBeginPlay
  ;[0.15 0.15 0.15 0.5] Add Timer Widget
  (bind _returnvalue (UserInterface|CreateWidget "/Game/Hypervoid/Blueprints/HUD/WBP_Timer.WBP_Timer_C"))
  (UserInterface|Viewport|AddtoViewport _returnvalue 0)
  (bind _output_get (Variables|Default|SetBackgroundMusic "/Game/Horrorscifimusickpack/CUES/Cue_The_sound_of_space.Cue_The_sound_of_space"))
  (Audio|PlaySoundatLocation _output_get "0, 0, 0" "0, 0, 0" 1.0 1.0 0.0 0 0 0 0))

(event EventTick
  (params (DeltaSeconds :type Float%20%28single-precision%29))
  (bind _returnvalue (Math|Random|RandomFloatinRange 5e+04 6e+04))
  ;[0.15 0.15 0.15 0.5] Set GamePlayTime
  (bind _output_get (Variables|Default|SetGamePlayTime (+ DeltaSeconds (Variables|Default|GetGamePlayTime))))
  (if (>= _output_get (Variables|Default|GetNextSpawnTime))
    ;[0.15 0.15 0.15 0.5] Update Next Spawn Time
    (bind _spawnperiod (CallFunction|CalculateSpawnPeriod 0.0))
    (Variables|Default|SetNextSpawnTime (+ _spawnperiod (Variables|Default|GetNextSpawnTime)))
    ;[0.15 0.15 0.15 0.5] Spawn Drones
    (bind _spawnamount (CallFunction|CalculateSpawnAmount (Variables|Default|GetGamePlayTime)))
    (for _index (range 1 _spawnamount)
      (CallFunction|SpawnDrone (Math|Random|RandomFloatinRange 6e+03 7.5e+03))
      (if (> (Variables|Default|GetGamePlayTime) 2.4e+02)
        (if (Variables|Default|GetMiddleBossFlag)
          (bind _outactors (Actor|GetAllActorsOfClass "/Game/Hypervoid/Blueprints/BP_MiddleBoss.BP_MiddleBoss_C"))
          (if (== (Utilities|Array|Length _outactors) 0)
            (bind _outactors_2 (Actor|GetAllActorsOfClass "/Game/Hypervoid/Blueprints/BP_LastBoss.BP_LastBoss_C"))
            (if (== (Utilities|Array|Length _outactors_2) 0)
              (CallFunction|SpawnLastBoss)
              (Variables|Default|SetBackgroundMusic "/Game/Free_Stylized_Beats/Cues/Sectors_120_BPM_wav_Cue.Sectors_120_BPM_wav_Cue")))
          (else
            (Variables|Default|SetMiddleBossFlag true)
            (CallFunction|SpawnMiddleBoss _returnvalue)
            (CallFunction|SpawnMiddleBoss _returnvalue)))))
    (else
      (if (> (Variables|Default|GetGamePlayTime) 2.4e+02)
        (if (Variables|Default|GetMiddleBossFlag)
          (bind _outactors_3 (Actor|GetAllActorsOfClass "/Game/Hypervoid/Blueprints/BP_MiddleBoss.BP_MiddleBoss_C"))
          (if (== (Utilities|Array|Length _outactors_3) 0)
            (bind _outactors_4 (Actor|GetAllActorsOfClass "/Game/Hypervoid/Blueprints/BP_LastBoss.BP_LastBoss_C"))
            (if (== (Utilities|Array|Length _outactors_4) 0)
              (CallFunction|SpawnLastBoss)
              (Variables|Default|SetBackgroundMusic "/Game/Free_Stylized_Beats/Cues/Sectors_120_BPM_wav_Cue.Sectors_120_BPM_wav_Cue")))
          (else
            (Variables|Default|SetMiddleBossFlag true)
            (CallFunction|SpawnMiddleBoss _returnvalue)
            (CallFunction|SpawnMiddleBoss _returnvalue)))))))

(fn ConstructionScript)

(fn SpawnDrone
  (params (DistanceFromPlayer :type Float%20%28double-precision%29))
  (bind _returnvalue (Math|Random|RandomUnitVector))
  (bind _returnvalue_2 (Game|GetPlayerCharacter 0))
  (bind _returnvalue_3 (Transformation|GetActorLocation _returnvalue_2))
  (bind _returnvalue_4 (* _returnvalue DistanceFromPlayer))
  (Game|SpawnActorfromClass "/Game/Hypervoid/Blueprints/BP_Drone.BP_Drone_C" (Math|Transform|MakeTransform (+ _returnvalue_4 _returnvalue_3) (Math|Rotator|FindLookatRotation _returnvalue_4 _returnvalue_3) "1.000000,1.000000,1.000000") "Undefined" "MultiplyWithRoot" 0 0))

(fn CalculateSpawnPeriod
  (params (CurrentTime :type Float%20%28double-precision%29))
  (if (Math|Float|InRange(Float) CurrentTime 0.0 2.4e+02)
    (return (Math|Conversions|ToFloat(Integer) (+ (* (/ -3 16) (Math|Float|Square (/ CurrentTime 6e+01))) 10)))
    (elif (Math|Float|InRange(Float) CurrentTime 2.4e+02 3e+02 false)
      (return (+ (* 6.5 (Math|Float|Square (- (/ CurrentTime 6e+01) 5.0))) 0.5))
      (else
        ;[0.15 0.15 0.15 0.5] y = 1 (x > 5)
        (return 1.0)))))

(fn CalculateSpawnAmount
  (params (CurrentTime :type Float%20%28double-precision%29))
  (if (Math|Float|InRange(Float) CurrentTime 0.0 2.4e+02)
    (return (Math|Float|Ceil (Math|Conversions|ToFloat(Integer) (+ (* (/ 9 16) (Math|Float|Square (/ CurrentTime 6e+01))) 1))))
    (elif true
      (return (Math|Float|Ceil (+ (* -5.0 (Math|Float|Square (- (/ CurrentTime 6e+01) 5.0))) 15.0)))
      (else
        ;[0.15 0.15 0.15 0.5] y = 15 (x > 5)
        (return 15)))))

(fn SpawnMiddleBoss
  (params (DistanceFromPlayer :type Float%20%28double-precision%29))
  (Game|SpawnActorfromClass "/Game/Hypervoid/Blueprints/BP_MiddleBoss.BP_MiddleBoss_C" (Math|Transform|MakeTransform (+ (* (Math|Random|RandomUnitVector) DistanceFromPlayer) (Transformation|GetActorLocation (Game|GetPlayerCharacter 0))) "0, 0, 0" "1.000000,1.000000,1.000000") "Undefined" "MultiplyWithRoot" 0 0))

(fn SpawnLastBoss
  (bind _returnvalue (Game|GetPlayerCharacter 0))
  (Game|SpawnActorfromClass "/Game/Hypervoid/Blueprints/BP_LastBoss.BP_LastBoss_C" (Math|Transform|MakeTransform (+ (Transformation|GetActorLocation _returnvalue) (* (Transformation|GetActorForwardVector _returnvalue) 5e+05)) "0, 0, 0" "2500.000000,2500.000000,2500.000000") "Undefined" "MultiplyWithRoot" 0 0))