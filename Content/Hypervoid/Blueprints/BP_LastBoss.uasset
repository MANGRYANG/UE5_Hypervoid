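; BP_LastBoss is the final boss of a survivors-like mode; its defeat wins the game.
; On BeginPlay it adds a directional light, has the game mode spawn two middle bosses, and starts a looping timer that spawns three more each cycle.
; Tick turns it toward the player until Health is depleted.
; It then explodes with an effect and sound and replaces all widgets with the win screen, showing the mouse cursor.
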(event Custom|SpawnThreeMiddleBoss
  (bind _asbp_survivors_like (Utilities|Casting|CastToBP_SurvivorsLike (Game|GetGameMode)))
  (for _index (range 0 2)
    (Default|SpawnMiddleBoss _asbp_survivors_like (Math|Random|RandomFloatinRange 5e+04 6e+04))))

(event EventTick
  (params (DeltaSeconds :type Float%20%28single-precision%29))
  (if (<= (Variables|Default|GetHealth) 0)
    (CallFunction|Explode)
    (CallFunction|WinGame)
    (else
      (Transformation|SetActorRotation (Math|Rotator|FindLookatRotation (Transformation|GetActorLocation) (Transformation|GetActorLocation (Game|GetPlayerCharacter 0)))))))

(event EventBeginPlay
  (bind _returnvalue (Math|Random|RandomFloatinRange 5e+04 6e+04))
  (AddComponent|AddDirectionalLightComponent false)
  (bind _asbp_survivors_like (Utilities|Casting|CastToBP_SurvivorsLike (Game|GetGameMode)))
  (Default|SpawnMiddleBoss _asbp_survivors_like _returnvalue)
  (Default|SpawnMiddleBoss _asbp_survivors_like _returnvalue)
  (Utilities|Time|SetTimerbyFunctionName 0 "SpawnThreeMiddleBoss" 1e+02 true))

(fn ConstructionScript)

(fn Explode
  (LocalVariables|SetExplode%20Point (Transformation|GetActorLocation))
  (Actor|DestroyActor)
  (Effects|SpawnEmitteratLocation "/Game/FXVarietyPack/Particles/P_ky_hit1.P_ky_hit1" (LocalVariables|GetExplode%20Point) (Math|Random|RandomRotator false) "10.000000,10.000000,10.000000")
  (Audio|PlaySoundatLocation "/Game/Sci-Fi_Shots_Pack2_Game_Of_Weapons/Cue/SciFi_Shot_P2__187__Cue.SciFi_Shot_P2__187__Cue" (Transformation|GetWorldLocation (Variables|/Script/Engine.Actor|GetRootComponent (Game|GetPlayerCharacter 0))) "0, 0, 0" 15.0 1.0 0.0 0 0 0 0))

(fn WinGame
  (Viewport|RemoveAllWidgets)
  (bind _returnvalue (UserInterface|CreateWidget "/Game/Hypervoid/Blueprints/HUD/WBP_WinGame.WBP_WinGame_C"))
  (UserInterface|Viewport|AddtoViewport _returnvalue 0)
  (Variables|/Script/Engine.PlayerController|SetbShowMouseCursor (Game|GetPlayerController (Variables|/Script/Engine.Pawn|GetPlayerState (Game|GetPlayerCharacter 0))) true))