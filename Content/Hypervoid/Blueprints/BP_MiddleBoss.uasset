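; BP_MiddleBoss is a suicide-bomber mid-boss that tumbles on a random axis and homes in on the player.
; Tick interpolates it toward the player until within 1000 units, then adjusts its spin, waits three seconds, explodes and calls Attacked on BP_Player.
; Zero health also triggers Explode, which destroys it with particles and sound played at the player's position.
; DropExpPoint adds EXP to the player but is not called here.
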(event EventTick
  (params (DeltaSeconds :type Float%20%28single-precision%29))
  (if (<= (Variables|Default|GetHealth) 0)
    (CallFunction|Explode)
    (else
      (Transformation|SetActorRotation (Math|Rotator|CombineRotators (Transformation|GetActorRotation) (* (Math|Conversions|RotationFromXVector (Variables|Default|GetRotation)) (Variables|Default|GetRotationSpeed))))
      (if (> (Math|Vector|Distance(Vector) (Transformation|GetActorLocation) (Transformation|GetActorLocation (Game|GetPlayerCharacter 0))) 1e+03)
        (Transformation|SetActorLocation (Math|Interpolation|VInterpTo (Transformation|GetActorLocation) (Transformation|GetActorLocation (Game|GetPlayerCharacter 0)) (Utilities|Time|GetWorldDeltaSeconds) (* (Variables|Default|GetVelocity) 0.1)) false false)
        (else
          (Variables|Default|SetRotationSpeed (Math|Interpolation|FInterpTo 0.01 1.0 DeltaSeconds 3.0))
          (Utilities|FlowControl|Delay 3.0)
          (CallFunction|Explode)
          (bind _asbp_player (Utilities|Casting|CastToBP_Player (Game|GetPlayerCharacter 0)))
          (Default|Attacked _asbp_player (Variables|Default|GetDamage)))))))

(event EventBeginPlay
  (Variables|Default|SetRotation (Math|Rotator|GetRotationXVector (Math|Random|RandomRotator false))))

(fn ConstructionScript)

(fn Explode
  (LocalVariables|SetExplode%20Point (Transformation|GetActorLocation))
  (Actor|DestroyActor)
  (Effects|SpawnEmitteratLocation "/Game/FXVarietyPack/Particles/P_ky_explosion.P_ky_explosion" (LocalVariables|GetExplode%20Point) (Math|Random|RandomRotator false) "10.000000,10.000000,10.000000")
  (Audio|PlaySoundatLocation "/Game/Free_Sounds_Pack/cue/Explosion_Large_1-1_Cue.Explosion_Large_1-1_Cue" (Transformation|GetWorldLocation (Variables|/Script/Engine.Actor|GetRootComponent (Game|GetPlayerCharacter 0))) "0, 0, 0" 15.0 1.0 0.0 0 0 0 0))

(fn DropExpPoint
  (bind _asbp_player (Utilities|Casting|CastToBP_Player (Game|GetPlayerCharacter 0)))
  (Variables|/Game/Hypervoid/Blueprints/BP_Player.BP_Player_C|SetEXP _asbp_player (+ (Variables|/Game/Hypervoid/Blueprints/BP_Player.BP_Player_C|GetEXP _asbp_player) (Variables|Default|GetDropEXP))))